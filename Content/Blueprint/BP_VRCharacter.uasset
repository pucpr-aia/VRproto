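; VR player character that lets either hand move or resize objects, depending on CurrentAction.
; Move line-traces from the hand, holds the hit component with a PhysicsHandle that always follows the right hand, and notifies its owner on release.
; Resize traces for BPI_Interactions actors, stores one per hand and sends grab and pinch-press messages.
; Tick also has J/K keys that nudge the right hand sideways.
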(event EventBeginPlay)

(event Collision|EventActorBeginOverlap
  (params (OtherActor :type Actor%20Object%20Reference)))

(event EventTick
  (params (DeltaSeconds :type Float%20%28single-precision%29))
  (bind _righthand (Variables|Default|GetRightHand))
  (bind _righthand_2 (Variables|Default|GetRightHand))
  (if (Variables|Default|GetIsGrabbing)
    (Physics|Components|PhysicsHandle|SetTargetLocation (Variables|Default|GetPhysicsHandle) (+ (Transformation|GetWorldLocation (Variables|Default|GetRightHandSphere)) (* (Math|Vector|GetForwardVector (Transformation|GetWorldRotation (Variables|Default|GetRightHandSphere))) (Variables|Default|GetInitDist)))))
  (if (Game|Player|IsInputKeyDown (Game|GetPlayerController 0) "K")
    (Transformation|SetRelativeLocation _righthand_2 (Math|Vector|MakeVector 6e+01 (+ (.y (Variables|/Script/Engine.SceneComponent|GetRelativeLocation _righthand_2)) 1.0) -25.0) false false)
    (elif (Game|Player|IsInputKeyDown (Game|GetPlayerController 0) "J")
      (Transformation|SetRelativeLocation _righthand (Math|Vector|MakeVector 6e+01 (- (.y (Variables|/Script/Engine.SceneComponent|GetRelativeLocation _righthand)) 1.0) -25.0) false false))))

(event Input|ActionEvents|InputActionGrabRight
  (params (Key :type Key%20Structure :default "None"))
  (:Pressed
    (switch Utilities|FlowControl|Switch|SwitchonETypes (Variables|Default|GetCurrentAction)
      (:NewEnumerator0
        (CallFunction|GrabMove true (Variables|Default|GetRightHandSphere)))
      (:NewEnumerator1
        (CallFunction|UpdatePointer (Variables|Default|GetRightHandSphere) "HandRight" true)
        (bind _righthitactor (Variables|Default|GetRightHitActor)
          (:then
            (Class|BPIInteractions|PrimaryPinchPressed(Message) _righthitactor (Variables|Default|GetRightHandSphere)))
          (:else)))))
  (:Released
    (switch Utilities|FlowControl|Switch|SwitchonETypes (Variables|Default|GetCurrentAction)
      (:NewEnumerator0
        (CallFunction|GrabMove false (Variables|Default|GetRightHandSphere)))
      (:NewEnumerator1
        (CallFunction|UpdatePointer (Variables|Default|GetRightHandSphere) "HandRight" false)
        (bind _righthitactor_2 (Variables|Default|GetRightHitActor)
          (:then
            (Class|BPIInteractions|PrimaryPinchReleased(Message) _righthitactor_2 (Variables|Default|GetRightHandSphere)))
          (:else))))))

(event Input|ActionEvents|InputActionGrabLeft
  (params (Key :type Key%20Structure :default "None"))
  (:Pressed
    (switch Utilities|FlowControl|Switch|SwitchonETypes (Variables|Default|GetCurrentAction)
      (:NewEnumerator0
        (CallFunction|GrabMove true (Variables|Default|GetLeftHandSphere)))
      (:NewEnumerator1
        (CallFunction|UpdatePointer (Variables|Default|GetLeftHandSphere) "HandLeft" true)
        (bind _lefthitactor (Variables|Default|GetLeftHitActor)
          (:then
            (Class|BPIInteractions|PrimaryPinchPressed(Message) _lefthitactor (Variables|Default|GetLeftHandSphere)))
          (:else)))))
  (:Released
    (switch Utilities|FlowControl|Switch|SwitchonETypes (Variables|Default|GetCurrentAction)
      (:NewEnumerator0
        (CallFunction|GrabMove false (Variables|Default|GetLeftHandSphere)))
      (:NewEnumerator1
        (CallFunction|UpdatePointer (Variables|Default|GetLeftHandSphere) "HandLeft" false)
        (bind _lefthitactor_2 (Variables|Default|GetLeftHitActor)
          (:then
            (Class|BPIInteractions|PrimaryPinchReleased(Message) _lefthitactor_2 (Variables|Default|GetLeftHandSphere)))
          (:else))))))

(fn ConstructionScript)

(fn GrabMove
  (params (Pressed :type Boolean) (Sphere :type Scene%20Component%20Object%20Reference))
  (bind _returnvalue (Transformation|GetWorldLocation Sphere))
  (if Pressed
    (if (not (Variables|Default|GetIsGrabbing))
      (Variables|Default|SetIsGrabbing true)
      (bind (_outhit _returnvalue_2) (Collision|LineTraceByChannel _returnvalue (+ _returnvalue (* (Math|Vector|GetForwardVector (Transformation|GetWorldRotation Sphere)) 5e+02)) "TraceTypeQuery1" false 0 "Persistent"))
      (if _returnvalue_2
        (Variables|Default|SetHit%20Component (.HitComponent (Collision|BreakHitResult _outhit)))
        (Physics|SetSimulatePhysics (Variables|Default|GetHit%20Component) true)
        (Physics|Components|PhysicsHandle|GrabComponentatLocationwithRotation (Variables|Default|GetPhysicsHandle) (Variables|Default|GetHit%20Component) "None" (Transformation|GetWorldLocation (Variables|Default|GetHit%20Component)) "0, 0, 0")
        (Variables|Default|SetInitDist (Math|Vector|Distance(Vector) (Transformation|GetWorldLocation (Variables|Default|GetRightHandSphere)) (Transformation|GetWorldLocation (Variables|Default|GetHit%20Component))))))
    (elif (Variables|Default|GetIsGrabbing)
      (Variables|Default|SetIsGrabbing false)
      (Variables|Default|GetHit%20Component
        (:then
          (Physics|SetSimulatePhysics (Variables|Default|GetHit%20Component) false)
          (Class|BPIInteractions|Release(Message) (Components|GetOwner (Variables|Default|GetHit%20Component)) (Variables|Default|GetHit%20Component))
          (Variables|Default|SetHit%20Component 0)
          (Physics|Components|PhysicsHandle|ReleaseComponent (Variables|Default|GetPhysicsHandle)))
        (:else)))))

(fn UpdatePointer
  (params (Input :type Scene%20Component%20Object%20Reference) (Hand :type EOculusHandType%20Enum :default "None") (Pressed :type Boolean))
  (bind _returnvalue (Transformation|GetWorldLocation Input))
  (if Pressed
    (bind (_outhit _returnvalue_2) (Collision|LineTraceByChannel _returnvalue (+ _returnvalue (* (Math|Vector|GetForwardVector Input) 1e+03)) "TraceTypeQuery1" false 0 "None"))
    (if _returnvalue_2
      (if (Utilities|DoesObjectImplementInterface (.HitActor (Collision|BreakHitResult _outhit)) "/Game/Blueprint/BPI_Interactions.BPI_Interactions_C")
        (switch Utilities|FlowControl|Switch|SwitchonEOculusHandType Hand
          (:HandLeft
            (bind _output_get (Variables|Default|SetLeftHitActor (.HitActor (Collision|BreakHitResult _outhit))))
            (Class|BPIInteractions|Grab(Message) _output_get (Variables|Default|GetLeftHandSphere)))
          (:HandRight
            (bind _output_get_2 (Variables|Default|SetRightHitActor (.HitActor (Collision|BreakHitResult _outhit))))
            (Class|BPIInteractions|Grab(Message) _output_get_2 (Variables|Default|GetRightHandSphere))))))
    (else
      (switch Utilities|FlowControl|Switch|SwitchonEOculusHandType Hand
        (:HandLeft
          (Variables|Default|SetLeftHitActor 0))
        (:HandRight
          (Variables|Default|SetRightHitActor 0))))))