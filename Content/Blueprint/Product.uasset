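; Product actor that can be scaled with a two-handed pinch gesture, likely for VR or hand tracking.
; It tracks up to two pinching hands; when the second pinches, it stores start distance and scale and enables Tick.
; Tick smoothly interpolates a clamped, uniform scale from the change in hand distance.
; Release prints a debug string and destroys the passed component if outside Box; Grab is empty.
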(event EventBeginPlay)

(event Collision|EventActorBeginOverlap
  (params (OtherActor :type Actor%20Object%20Reference)))

(event EventTick
  (params (DeltaSeconds :type Float%20%28single-precision%29))
  (Variables|Default|GetFirstHand
    (:then
      (Variables|Default|GetSecondHand
        (:then
          (bind _returnvalue (CallFunction|CalculateNewScale))
          (Transformation|SetActorScale3D _returnvalue))
        (:else)))
    (:else)))

(event EventGrab
  (params (Scene%20Component :type Scene%20Component%20Object%20Reference)))

(event EventRelease
  (params (Component :type Primitive%20Component%20Object%20Reference))
  (Development|PrintString "Hello")
  (if (not (Class|PrimitiveComponent|IsOverlappingComponent (Variables|Default|GetBox) Component))
    (Components|DestroyComponent Component)))

(event EventPrimaryPinchPressed
  (params (Hand :type Scene%20Component%20Object%20Reference))
  (Variables|Default|GetFirstHand
    (:then
      (Variables|Default|SetSecondHand Hand)
      (Variables|Default|SetStartHandDistance (CallFunction|GetHandDistance))
      (Variables|Default|SetStart%20Scale (Transformation|GetActorScale3D))
      (Actor|Tick|SetActorTickEnabled true))
    (:else
      (Variables|Default|SetFirstHand Hand))))

(event EventPrimaryPinchReleased
  (params (Hand :type Scene%20Component%20Object%20Reference))
  (if (== Hand (Variables|Default|GetSecondHand))
    (Variables|Default|SetSecondHand 0)
    (elif (== Hand (Variables|Default|GetFirstHand))
      (bind _secondhand (Variables|Default|GetSecondHand)
        (:then
          (Variables|Default|SetFirstHand _secondhand)
          (Variables|Default|SetSecondHand 0))
        (:else
          (Variables|Default|SetFirstHand 0)))
      (Actor|Tick|SetActorTickEnabled false))))

(fn ConstructionScript)

(fn GetHandDistance
  (Variables|Default|GetFirstHand
    (:then
      (Variables|Default|GetSecondHand
        (:then
          (return (Math|Float|Absolute(Float) (Math|Vector|VectorLength (- (Transformation|GetWorldLocation (Variables|Default|GetFirstHand)) (Transformation|GetWorldLocation (Variables|Default|GetSecondHand)))))))
        (:else)))
    (:else)))

(fn CalculateNewScale
  (bind _output_get (LocalVariables|SetDistance%20Diff (/ (- (CallFunction|GetHandDistance) (Variables|Default|GetStartHandDistance)) (Variables|Default|GetHandDistanceDivider))))
  (bind _output_get_2 (LocalVariables|SetModifiedScale (+ (Variables|Default|GetStart%20Scale) _output_get)))
  (if (!= (Math|Float|Clamp(Float) (.X (Math|Vector|BreakVector _output_get_2)) (Variables|Default|GetMinScale) (Variables|Default|GetMaxScale)) 0.0)
    (return (Math|Interpolation|VInterpTo (Transformation|GetActorScale3D) (Math|Vector|MakeVector (Math|Float|Clamp(Float) (.X (Math|Vector|BreakVector _output_get_2)) (Variables|Default|GetMinScale) (Variables|Default|GetMaxScale)) (Math|Float|Clamp(Float) (.X (Math|Vector|BreakVector _output_get_2)) (Variables|Default|GetMinScale) (Variables|Default|GetMaxScale)) (Math|Float|Clamp(Float) (.X (Math|Vector|BreakVector _output_get_2)) (Variables|Default|GetMinScale) (Variables|Default|GetMaxScale))) (Utilities|Time|GetWorldDeltaSeconds) (Variables|Default|GetScaleSpeed)))
    (else
      (return (Transformation|GetActorScale3D)))))